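; BPEnemyCharacter is an enemy character Blueprint that carries a weapon and a health component oriented toward the player.
; On BeginPlay it spawns a BP_weapon, stores it as Weapon and snaps it to the mesh's Hand_r socket.
; Every Tick it rotates the Healht component in world space to face player character 0, billboard-style.
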(event EventBeginPlay
  (bind _returnvalue (Game|SpawnActorfromClass "/Game/Blueprints/BP_weapon.BP_weapon_C" (Math|Transform|MakeTransform "0, 0, 0") "AlwaysSpawn" 0 0))
  (bind _output_get (Variables|Default|SetWeapon _returnvalue))
  (Transformation|AttachComponentToComponent _output_get (Variables|Character|GetMesh) "Hand_r" "SnapToTarget" "SnapToTarget" "SnapToTarget" true))

(event Collision|EventActorBeginOverlap
  (params (OtherActor :type Actor%20Object%20Reference)))

(event EventTick
  (params (DeltaSeconds :type Float%20%28single-precision%29))
  (bind _healht (Variables|Default|GetHealht))
  (Transformation|SetWorldRotation _healht (Math|Rotator|FindLookatRotation (Transformation|GetWorldLocation _healht) (Transformation|GetActorLocation (Game|GetPlayerCharacter 0))) false false))

(fn ConstructionScript)